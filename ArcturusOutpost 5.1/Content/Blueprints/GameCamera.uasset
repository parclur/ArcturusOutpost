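; GameCamera is a third-person camera actor that orbits and follows the player's ThirdPersonCharacter.
; Each tick it clamps the character's mouse input, rotates its offset around the character's JumpLoc, eases toward that position and looks at that point with a pitch offset.
; A visibility line trace from the character then snaps the camera to any blocking hit.
; Grounded-only follow logic exists but never runs, and a debug print shows the mouse delta.
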(event `self.ReceiveBeginPlay`
  (set `self.mousePos` (0.0 0.0 0.0))
  ;[1 1 1] if the player character is not assigned then assign it
  (if (not (`KismetSystemLibrary.IsValid` (`self.PlayerCharacter`)))
    (bind _asthird_person_character (cast `/Game/Blueprints/ThirdPersonCharacter` (`GameplayStatics.GetPlayerCharacter` 0)))
    (set `self.PlayerCharacter` _asthird_person_character))
  (set `self.PlayerDiff` (- (`SceneComponent.K2_GetComponentLocation` (`self.CameraComponent`)) (.location (`self.GetTransform` (`self.PlayerCharacter`))))))

(event `self.ReceiveTick`
  (params (DeltaSeconds :type "Float (single-precision)"))
  ;[1 1 1] reset the player character if respawned or not previously attached
  (`KismetSystemLibrary.PrintString` (`KismetStringLibrary.Conv_VectorToString` (`self.deltaMouse`)) true true (struct :`R` 1.0 :`G` 1.0 :`A` 1.0) 0.01)
  (if (not (`KismetSystemLibrary.IsValid` (`self.PlayerCharacter`)))
    (bind _asthird_person_character (cast `/Game/Blueprints/ThirdPersonCharacter` (`GameplayStatics.GetPlayerCharacter` 0)))
    (set `self.PlayerCharacter` _asthird_person_character))
  (`self.UpdateMouseDelta`)
  (`self.RotateCamera`)
  (`self.TraceForCameraCollision`))

(event `CheckForFollowCharacter`
  ;[1 1 1] Move the camera only when the character is grounded so we dont follow during the jumping
  ;;[1 1 1] FollowCharacter Area
  (`self.K2_SetActorTransform` (`KismetMathLibrary.MakeTransform` (+ (`/Game/Blueprints/ThirdPersonCharacter.JumpLoc` (`self.PlayerCharacter`)) (* (* (- (`SceneComponent.K2_GetComponentLocation` (`self.CameraComponent`)) (`/Game/Blueprints/ThirdPersonCharacter.JumpLoc` (`self.PlayerCharacter`))) (`self.CamDistance`)) (* (`GameplayStatics.GetWorldDeltaSeconds`) (`self.CamMoveSpeed`)))) (.rotation (`self.GetTransform` self)) (.scale (`self.GetTransform` self)))))

(event `TraceForCameraCollision`
  (bind _playercharacter (`self.PlayerCharacter`))
  ;[1 1 1] Making the camera move closer to the character if there is in object in the waY
  (bind (_outhit _returnvalue) (`KismetSystemLibrary.LineTraceSingle` (.location (`self.GetTransform` _playercharacter)) (`SceneComponent.K2_GetComponentLocation` (`self.CameraComponent`)) "TraceTypeQuery1" false (`|MakeArray` _playercharacter self :!type "Actor Object Reference")))
  (if _returnvalue
    (`self.K2_SetActorTransform` (`KismetMathLibrary.MakeTransform` (`.Location` (`GameplayStatics.BreakHitResult` _outhit)) (`self.K2_GetActorRotation` self)) false true)))

(event `UpdateMouseDelta`
  (bind _playercharacter (`self.PlayerCharacter`))
  ;[1 1 1] Updating the mouse pos and delta for rotation
  (bind _output_get (set `self.deltaMouse` (`KismetMathLibrary.MakeVector` (`KismetMathLibrary.FClamp` (`/Game/Blueprints/ThirdPersonCharacter.mouseInputX` _playercharacter) -9.9 9.9) (`KismetMathLibrary.FClamp` (`/Game/Blueprints/ThirdPersonCharacter.mouseInputY` _playercharacter) -9.9 9.9))))
  (set `self.mousePos` (+ _output_get (`self.mousePos`))))

(event `RotateCamera`
  (bind _camdistance (`self.CamDistance`))
  (bind _returnvalue (`SceneComponent.K2_GetComponentLocation` (`self.CameraComponent`)))
  (bind _jumploc (`/Game/Blueprints/ThirdPersonCharacter.JumpLoc` (`self.PlayerCharacter`)))
  (bind _returnvalue_2 (- (`SceneComponent.K2_GetComponentLocation` (`self.CameraComponent`)) _jumploc))
  ;[1 1 1] Trying to rotate the camera
  (`self.K2_SetActorLocationAndRotation` (+ (* (- (+ _jumploc (* (`KismetMathLibrary.Normal` (`KismetMathLibrary.RotateAngleAxis` _returnvalue_2 (* (.x (`self.deltaMouse`)) (`self.CamRotSpeed`) (`GameplayStatics.GetWorldDeltaSeconds`)) (`self.GetActorUpVector` (`self.PlayerCharacter`)))) _camdistance) (* (`KismetMathLibrary.Normal` (`KismetMathLibrary.RotateAngleAxis` _returnvalue_2 (* (.y (`self.deltaMouse`)) (`self.CamPitchSpeed`) (`GameplayStatics.GetWorldDeltaSeconds`)) (`self.GetActorRightVector` self))) _camdistance)) _returnvalue) (`GameplayStatics.GetWorldDeltaSeconds`) (`self.CamMoveSpeed`)) _returnvalue) (`KismetMathLibrary.MakeRotator` (.roll (`KismetMathLibrary.FindLookAtRotation` (`SceneComponent.K2_GetComponentLocation` (`self.CameraComponent`)) (+ (`/Game/Blueprints/ThirdPersonCharacter.JumpLoc` (`self.PlayerCharacter`)) (0.0 0.0 10.0)))) (+ (.pitch (`KismetMathLibrary.FindLookAtRotation` (`SceneComponent.K2_GetComponentLocation` (`self.CameraComponent`)) (+ (`/Game/Blueprints/ThirdPersonCharacter.JumpLoc` (`self.PlayerCharacter`)) (0.0 0.0 10.0)))) 10.0) (.yaw (`KismetMathLibrary.FindLookAtRotation` (`SceneComponent.K2_GetComponentLocation` (`self.CameraComponent`)) (+ (`/Game/Blueprints/ThirdPersonCharacter.JumpLoc` (`self.PlayerCharacter`)) (0.0 0.0 10.0)))))))

(fn `UserConstructionScript`)