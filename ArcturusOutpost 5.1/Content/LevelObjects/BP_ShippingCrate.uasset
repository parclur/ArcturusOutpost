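; A shipping crate level object that moves between its placed position and a configurable MoveToPos offset.
; The construction script gives its InterpToMovement component two relative control points, the origin and MoveToPos.
; Movement activates on BeginPlay unless BoltCrankActivated is set.
; The MoveShippingCrates event also activates the movement, letting crank-activated crates start on an external call.
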(event `self.ReceiveBeginPlay`
  (if (not (`self.BoltCrankActivated?`))
    (`ActorComponent.Activate` (`self.InterpToMovement`) false)))

(event `MoveShippingCrates`
  (`ActorComponent.Activate` (`self.InterpToMovement`) false))

(fn `UserConstructionScript`
  (bind _interptomovement (`self.InterpToMovement`))
  (`InterpToMovementComponent.AddControlPointPosition` _interptomovement (0.0 0.0 0.0) true)
  (`InterpToMovementComponent.AddControlPointPosition` _interptomovement (`self.MoveToPos`) true))