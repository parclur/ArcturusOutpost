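; BP_Smasher is a level object that repeatedly moves down and up along Z as a stamping smasher.
; On BeginPlay it records its start location and a lowered height a fixed distance below it.
; The Smasher timeline interpolates the actor's height between the two.
; When the timeline finishes, it waits for StampingDelay and replays from the start, looping indefinitely.
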(event `self.ReceiveBeginPlay`
  (bind _output_get (set `self.StartLocation` (`self.K2_GetActorLocation`)))
  (bind _output_get_2 (set `self.StartingHeight` (.z _output_get)))
  (set `self.LoweredHeight` (- _output_get_2 400.0))
  (bind (_direction _newtrack_1) (`Timeline|Smasher` :!label _label)
    (:`Update`
      (`self.K2_SetActorLocation` (`KismetMathLibrary.MakeVector` (.x (`self.StartLocation`)) (.y (`self.StartLocation`)) (`KismetMathLibrary.Lerp` (`self.StartingHeight`) (`self.LoweredHeight`) _newtrack_1))))
    (:`Finished`
      (`KismetSystemLibrary.Delay` (`self.StampingDelay`))
      (goto _label :!via `PlayFromStart`))))

(fn `UserConstructionScript`)