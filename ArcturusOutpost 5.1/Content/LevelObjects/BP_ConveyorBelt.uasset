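; Conveyor belt level object that carries overlapping actors along and can be raised into a new position.
; Each tick it offsets every actor in its Box along the Arrow's forward vector at Speed, without sweeping.
; If MoveConveyor is set, RaiseConveyor plays a timeline that lerps height and roll toward raised values, applying target pitch and yaw directly.
; The construction script inversely scales the Arrow so it stays unstretched.
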(event `self.ReceiveTick`
  (params (DeltaSeconds :type "Float (single-precision)"))
  ;[1 1 1] Moves the player forward like on a conveyor belt
  (for _array_element (`PrimitiveComponent.GetOverlappingActors` (`self.Box`) null)
    (`self.K2_AddActorWorldOffset` _array_element (* (`KismetMathLibrary.GetForwardVector` (`SceneComponent.K2_GetComponentRotation` (`self.Arrow`))) (* DeltaSeconds (`self.Speed`))) false false)))

(event `RaiseConveyor`
  (if (`self.Move Conveyor?`)
    (set `self.Start Location` (`self.K2_GetActorLocation`))
    (bind (_direction _z_location _y_rotation) (`Timeline|Raise`)
      (:`Update`
        (`self.K2_SetActorLocation` (`KismetMathLibrary.MakeVector` (.x (`self.Start Location`)) (.y (`self.Start Location`)) (`KismetMathLibrary.Lerp` (.z (`self.Start Location`)) (`self.RaisedHeight`) _z_location)))
        (`self.K2_SetActorRotation` (`KismetMathLibrary.MakeRotator` (`KismetMathLibrary.Lerp` (.roll (`self.Start Rotation`)) (.roll (`self.Raised Rotation`)) _y_rotation) (.pitch (`self.Raised Rotation`)) (.yaw (`self.Raised Rotation`))))))))

(fn `UserConstructionScript`
  ;[1 1 1] Keeps the conveyor direction arrow from getting stretched out
  (`SceneComponent.SetRelativeScale3D` (`self.Arrow`) (/ (1.0 1.0 1.0) (`self.GetActorScale3D`))))