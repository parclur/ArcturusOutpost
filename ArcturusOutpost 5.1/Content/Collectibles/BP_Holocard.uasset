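; BP_Holocard is a collectible actor that bobs and spins in place and destroys itself when any actor overlaps it.
; On BeginPlay it caches its starting transform, then a timeline lerps height up to a small offset and yaw from the starting value toward 360 degrees.
; The timeline replays from the start through a zero-length delay whenever it finishes, and no score or inventory logic runs on pickup.
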(event `self.ReceiveBeginPlay`
  (bind _output_get (set `self.StartLocation` (`self.K2_GetActorLocation`)))
  (set `self.EndLocation` (+ (.z _output_get) 20.0))
  (set `self.StartRotation` (`self.K2_GetActorRotation`))
  (bind (_direction _bobbing _spinning) (`Timeline|Timeline` :!label _label)
    (:`Update`
      (`self.K2_SetActorLocationAndRotation` (`KismetMathLibrary.MakeVector` (.x (`self.StartLocation`)) (.y (`self.StartLocation`)) (`KismetMathLibrary.Lerp` (.z (`self.StartLocation`)) (`self.EndLocation`) _bobbing)) (`KismetMathLibrary.MakeRotator` (.roll (`self.StartRotation`)) (.pitch (`self.StartRotation`)) (`KismetMathLibrary.Lerp` (.yaw (`self.StartRotation`)) 360.0 _spinning))))
    (:`Finished`
      (`KismetSystemLibrary.Delay` 0.0)
      (goto _label :!via `PlayFromStart`))))

(event `self.ReceiveActorBeginOverlap`
  (params (OtherActor :type "Actor Object Reference"))
  (`self.K2_DestroyActor`))

(fn `UserConstructionScript`)