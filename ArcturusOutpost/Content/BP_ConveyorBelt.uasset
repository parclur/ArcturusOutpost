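; BP_ConveyorBelt is a conveyor belt actor that carries third-person characters along its forward direction.
; Each tick it finds ThirdPersonCharacter actors overlapping its Box and offsets them by forward vector times Speed and delta time, without sweeping.
; The construction script counter-scales the Arrow by the inverse actor scale so the direction indicator stays undistorted when the belt is resized.
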(event `self.ReceiveTick`
  (params (DeltaSeconds :type "Float (single-precision)"))
  (for _array_element (`PrimitiveComponent.GetOverlappingActors` (`self.Box`) "/Game/ThirdPersonBP/Blueprints/ThirdPersonCharacter.ThirdPersonCharacter_C")
    (`self.K2_AddActorWorldOffset` _array_element (* (`KismetMathLibrary.GetForwardVector` (`self.K2_GetActorRotation`)) (* DeltaSeconds (`self.Speed`))) false false)))

(fn `UserConstructionScript`
  ;[1 1 1] Keeps the conveyor direction arrow from getting stretched out
  (`SceneComponent.SetRelativeScale3D` (`self.Arrow`) (/ (1.0 1.0 1.0) (`self.GetActorScale3D`))))