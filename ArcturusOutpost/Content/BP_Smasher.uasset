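; BP_Smasher is an actor that repeatedly stamps down and rises back, like a crusher obstacle.
; Tick moves it along local Z at separate down and up speeds, flipping Stamping between StartingHeight and 500 units below.
; StampingDelay holds it on reaching the top, then is zeroed, so only the first such pause uses it.
; StartingHeight relies on its variable value, as the construction-script assignment from Cube is disconnected.
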(event `self.ReceiveBeginPlay`)

(event `self.ReceiveTick`
  (params (DeltaSeconds :type "Float (single-precision)"))
  (bind (_returnvalue_x _returnvalue_y _returnvalue_z) (`KismetMathLibrary.BreakVector` (`self.K2_GetActorLocation`)))
  (bind (_returnvalue_x_2 _returnvalue_y_2 _returnvalue_z_2) (`KismetMathLibrary.BreakVector` (`self.K2_GetActorLocation`)))
  (bind (_returnvalue_x_3 _returnvalue_y_3 _returnvalue_z_3) (`KismetMathLibrary.BreakVector` (`self.K2_GetActorLocation`)))
  (bind (_returnvalue_x_4 _returnvalue_y_4 _returnvalue_z_4) (`KismetMathLibrary.BreakVector` (`self.K2_GetActorLocation`)))
  (if (`self.Stamping`)
    (if (> _returnvalue_z_2 (- (`self.StartingHeight`) 500.0))
      (`self.K2_AddActorLocalOffset` (`KismetMathLibrary.MakeVector` 0.0 0.0 (* (`GameplayStatics.GetWorldDeltaSeconds`) (`self.DownSpeed`))))
      (if (<= _returnvalue_z_3 (- (`self.StartingHeight`) 500.0))
        (set `self.Stamping` false)))
    (elif (< _returnvalue_z_4 (`self.StartingHeight`))
      (`self.K2_AddActorLocalOffset` (`KismetMathLibrary.MakeVector` 0.0 0.0 (* (`GameplayStatics.GetWorldDeltaSeconds`) (`self.Up_Speed`))))
      (if (>= _returnvalue_z (`self.StartingHeight`))
        (`KismetSystemLibrary.Delay` (`self.StampingDelay`))
        (set `self.Stamping` true)
        (set `self.StampingDelay` 0.0)))))

(fn `UserConstructionScript`)